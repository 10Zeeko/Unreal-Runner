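; Spawner actor that creates obstacles and birds for what appears to be an endless runner with a scrolling floor.
; It spawns a random obstacle class on BeginPlay and on each SpawnNewObstacle call, while a looping timer separately spawns birds at the same point.
; When Points is a multiple of five, obstacle speed rises up to a cap, and floor speed increases alongside it through a Material Parameter Collection.
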(event `self.ReceiveBeginPlay`
  (bind _obstaclesspeed (`self.ObstaclesSpeed`))
  (bind _floorspeed (`self.FloorSpeed`))
  (`|ExecutionSequence`
    (:`then_0`
      (`KismetSystemLibrary.K2_SetTimer` null "Timer" 8.0 true))
    (:`then_1`
      (`|SpawnActorFromClass` (`KismetArrayLibrary.Array_Random` (`self.Actors`)) (`KismetMathLibrary.MakeTransform` (2000.0 0.0 50.0)) "Undefined" "MultiplyWithRoot" null (2000.0 0.0 50.0) (-500.0 0.0 50.0) (`self.ObstaclesSpeed`) null :!label _label)
      (if (== (mod (stale `SpawnNewObstacle` Points) 5) 0)
        (if (< _obstaclesspeed 16.0)
          (set `self.ObstaclesSpeed` (+ _obstaclesspeed 0.25))
          (`KismetMaterialLibrary.SetVectorParameterValue` "/Game/Materials/FloorSpeed.FloorSpeed" "Speed" (make `LinearColor` _floorspeed 0.0 0.0 _floorspeed))
          (set `self.FloorSpeed` (+ (`self.FloorSpeed`) 0.003)))))))

(event `SpawnNewObstacle`
  (params (Points :type Integer))
  (goto _label))

(fn `Timer`
  (`|SpawnActorFromClass` "/Game/Obstacles/Bird.Bird_C" (`KismetMathLibrary.MakeTransform` (2000.0 0.0 50.0)) "Undefined" "MultiplyWithRoot" null (2000.0 0.0 200.0) (-500.0 0.0 50.0) (`self.ObstaclesSpeed`) null))

(fn `UserConstructionScript`)